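; Gesture component that detects shake, stir and pour motions from a tracked controller component while an item is held.
; While tracking, Tick derives velocity and speed, then runs the three gesture handlers.
; Shake times fast direction reversals, stir accumulates yaw around an externally set origin within a radius band, and pour scales flow by tilt from world up.
; Results are only printed as debug strings or kept in variables.
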(event `self.ReceiveTick`
  (params (DeltaSeconds :type "Float (single-precision)"))
  (bind _returnvalue (`SceneComponent.K2_GetComponentLocation` (`self.TrackedComponent`)))
  (bind _returnvalue_2 (/ (- _returnvalue (`self.LastLocation`)) (`self.Delta Seconds`)))
  ; Get Speed and other data from controller each tick
  (set `self.Delta Seconds` DeltaSeconds)
  (if (`self.bIsTracking`)
    (set `self.Velocity` _returnvalue_2)
    (set `self.Speed` (`KismetMathLibrary.VSize` _returnvalue_2))
    (set `self.LastLocation` _returnvalue)
    (`self.HandleShake`)
    (`self.HandleStir`)
    (`self.HandlePour`)))

(event `HandleShake`
  (bind _returnvalue (`KismetMathLibrary.Normal` (`self.Velocity`)))
  ; Update Status towards shake gesture
  (if (< (`self.Speed`) (`self.ShakeSpeedThreshold`))
    _
    (elif (`self.bHasLastShakeDir`)
      (if (< (`KismetMathLibrary.Dot_VectorVector` _returnvalue (`self.LastShakeDir`)) (`self.MinDirectionDot`))
        (set `self.ShakeAccumulatedTime` (+ (`self.ShakeAccumulatedTime`) (`self.Delta Seconds`)))
        (set `self.LastShakeDir` (stale _output_get))
        (if (>= (`self.ShakeAccumulatedTime`) (`self.RequiredShakeTime`))
          (`KismetSystemLibrary.PrintString` "Shake Gesture complete")
          (set `self.ShakeAccumulatedTime` 0.0)
          (set `self.bHasLastShakeDir` false)))
      (else
        (bind _output_get (set `self.LastShakeDir` _returnvalue))
        (set `self.bHasLastShakeDir` true)))))

(event `HandleStir`
  (bind (_currentdir2d_x _currentdir2d_y) (`KismetMathLibrary.BreakVector2D` (`self.currentDir2D`)))
  (bind (_lastlocaldir2d_x _lastlocaldir2d_y) (`KismetMathLibrary.BreakVector2D` (`self.LastLocalDir2D`)))
  (bind _returnvalue (`KismetMathLibrary.Conv_VectorToVector2D` (- (`SceneComponent.K2_GetComponentLocation` (`self.TrackedComponent`)) (`self.StirOriginWS`))))
  (if (and (`self.bIsTracking`) (`self.bHasStirContext`))
    (set `self.Offset2D` _returnvalue)
    (bind _output_get (set `self.StirRadius` (`KismetMathLibrary.VSize2D` _returnvalue)))
    (if (or (<= _output_get (`self.StirRadiusMin`)) (>= _output_get (`self.StirRadiusMax`)))
      _
      (elif (`self.bHasLastLocalDir`)
        (bind _output_get_2 (set `self.currDir3D` (`KismetMathLibrary.MakeVector` _currentdir2d_x _currentdir2d_y)))
        (bind _output_get_3 (set `self.lastDir3D` (`KismetMathLibrary.MakeVector` _lastlocaldir2d_x _lastlocaldir2d_y)))
        (bind _output_get_4 (set `self.currRot` (`KismetMathLibrary.MakeRotFromX` _output_get_2)))
        (bind _output_get_5 (set `self.lastRot` (`KismetMathLibrary.MakeRotFromX` _output_get_3)))
        (bind _output_get_6 (set `self.currYaw` (.yaw _output_get_4)))
        (bind _output_get_7 (set `self.prevYaw` (.yaw _output_get_5)))
        (bind _returnvalue_2 (- _output_get_6 _output_get_7))
        (set `self.deltaYaw` _returnvalue_2)
        (if (> _returnvalue_2 180.0)
          (set `self.deltaYaw` (- (`self.deltaYaw`) 360.0))
          (elif (< (`self.deltaYaw`) -180.0)
            (bind _output_get_8 (set `self.deltaYaw` (+ (`self.deltaYaw`) 360.0)))
            (bind _output_get_9 (set `self.angleDelta` (`KismetMathLibrary.Abs` _output_get_8)))
            (`KismetSystemLibrary.PrintString` (`KismetStringLibrary.Conv_DoubleToString` _output_get_9))
            (bind _output_get_10 (set `self.AccumulatedStirAngle` (+ (`self.AccumulatedStirAngle`) _output_get_9)))
            (set `self.LastLocalDir2D` (`self.currentDir2D`))
            (if (>= _output_get_10 (`self.RequiredStirAngle`))
              (`KismetSystemLibrary.PrintString` "STIR GESTURE COMPLETE")
              (set `self.AccumulatedStirAngle` 0.0)
              (set `self.bHasLastLocalDir` false))))
        (else
          (bind _output_get_11 (set `self.LastLocalDir2D` (`KismetMathLibrary.Normal2D` _returnvalue)))
          (set `self.currentDir2D` _output_get_11)
          (set `self.bHasLastLocalDir` true))))))

(event `HandlePour`
  (if (`self.bIsTracking`)
    (bind _output_get (set `self.HandUpWS` (`SceneComponent.GetUpVector` (`self.TrackedComponent`))))
    (set `self.angleDeg` (`KismetMathLibrary.RadiansToDegrees` (`KismetMathLibrary.Acos` (`KismetMathLibrary.Dot_VectorVector` (0.0 0.0 1.0) _output_get))))
    (if (and (not (`self.bIsPouring`)) (>= (`self.PourStartAngleDeg`) (`self.angleDeg`)))
      (set `self.bIsPouring` true)
      (`KismetSystemLibrary.PrintString` "pouring")
      (elif (and (`self.bIsPouring`) (<= (`self.PourStopAngleDeg`) (`self.angleDeg`)))
        (set `self.bIsPouring` false)
        (elif (`self.bIsPouring`)
          (bind _output_get_2 (set `self.tiltRange` (- (`self.MaxPourAngleDeg`) (`self.PourStartAngleDeg`))))
          (set `self.CurrentPourStrength ` (/ (`KismetMathLibrary.FClamp` (- (`self.angleDeg`) (`self.PourStartAngleDeg`)) 0.0 _output_get_2) (`self.tiltRange`)))
          (bind _output_get_3 (set `self.CurrentPourAmount` (+ (* (`self.PourFlowRate`) (`self.CurrentPourStrength `) (`self.Delta Seconds`)) (`self.CurrentPourAmount`))))
          (`KismetSystemLibrary.PrintString` (`KismetStringLibrary.Conv_DoubleToString` _output_get_3)))))))

(fn `ClearStirContext`
  (set `self.bHasStirContext` false))

(fn `SetStirContext`
  (params (OriginWS :type "Vector Structure") (RadiusMin :type "Float (double-precision)") (RadiusMax :type "Float (double-precision)"))
  (set `self.StirOriginWS` OriginWS)
  (set `self.StirRadiusMin` RadiusMin)
  (set `self.StirRadiusMax` RadiusMax)
  (set `self.bHasStirContext` true)
  (set `self.AccumulatedStirAngle` 0.0)
  (set `self.bHasLastLocalDir` false))

(fn `StartTracking`
  (params (HeldActor :type "Actor Object Reference"))
  (set `self.bIsTracking` true)
  (set `self.CurrentHeldActor` HeldActor)
  (set `self.LastLocation` (`Actor.K2_GetActorLocation` (`self.GetOwner`)))
  (set `self.Velocity` (0.0 0.0 0.0))
  (set `self.Speed` 0.0)
  (set `self.ShakeAccumulatedTime` 0.0)
  (set `self.bHasLastShakeDir` false)
  (set `self.RequiredStirAngle` 0.0)
  (set `self.bHasLastLocalDir` false))

(fn `StopTracking`
  (set `self.bIsTracking` false)
  (set `self.CurrentHeldActor` null))